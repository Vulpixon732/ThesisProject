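; Actor component that watches a BP_ActionChar owner, apparently an enemy, and records its combat performance against the player for scoring.
; BeginCombat and EndCombat toggle component tick, which accumulates time to kill while DealtDamageToPlayer totals damage inflicted.
; SendData passes the owner's class and combat data to the scoring agent cached from GM_Thesis, with debug prints throughout.
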(event Custom|BeginCombat
  (if (not (Class|ActorComponent|IsComponentTickEnabled))
    (Components|Tick|SetComponentTickEnabled true)
    (Development|PrintText "Combat started")))

(event Custom|SendData
  (bind _asbp_action_char (Utilities|Casting|CastToBP_ActionChar (Components|GetOwner)))
  (Default|ReceiveCombatData (Variables|Default|GetScoringAgent) (Utilities|GetClass _asbp_action_char) (Variables|Default|GetCombatData)))

(event Custom|EndCombat
  (if (Class|ActorComponent|IsComponentTickEnabled)
    (Components|Tick|SetComponentTickEnabled false)
    (Development|PrintText "Combat ended")))

(event EventBeginPlay
  (bind _asgm_thesis (Utilities|Casting|CastToGM_Thesis (Game|GetGameMode)))
  (Variables|Default|SetScoringAgent (Variables|/Game/Blueprints/GM_Thesis.GM_Thesis_C|GetAC_ScoringAgent _asgm_thesis)))

(event EventTick
  (params (DeltaSeconds :type Float%20%28single-precision%29))
  (Variables|Default|SetCombatData (Utilities|Struct|MakeS_CombatData (.damagereceived (Variables|Default|GetCombatData)) (+ (.timetokill (Variables|Default|GetCombatData)) DeltaSeconds)))
  (Development|PrintText (Utilities|Text|FormatText "Elapsed combat time: {x}" (.timetokill (Variables|Default|GetCombatData)))))

(fn DealtDamagetoPlayer
  (params (Damage :type Float%20%28double-precision%29))
  (Variables|Default|SetCombatData (Utilities|Struct|MakeS_CombatData (+ Damage (.damagereceived (Variables|Default|GetCombatData))) (.timetokill (Variables|Default|GetCombatData))))
  ;[1 1 1] DEBUG
  (Development|PrintText (Utilities|Text|FormatText "Total damage dealt: {x}" (.damagereceived (Variables|Default|GetCombatData)))))