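; Scoring agent component that records combat results per character class and carries them, with a point pool, across level transitions.
; ReceiveCombatData appends each record, with damage received and time to kill, to that class's entry, then debug-prints the class's history.
; BeginPlay restores data from GI_Thesis, using the starting pool on level zero, and copies the pool to a temporary one.
; EndPlay on a level transition increments the level counter and saves both back to the game instance.
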(event Custom|ReceiveCombatData
  (params (ActionCharacter :type BP%20Action%20Char%20Class%20Reference) (CombatData :type S%20Combat%20Data%20Structure))
  (CallFunction|SaveCombatData ActionCharacter CombatData)
  (Debug|DEBUGPrintCollectedCombatData ActionCharacter))

(event EventBeginPlay
  (Utilities|FlowControl|Sequence
    (:then_0
      ;[1 1 1] Set Game Instance reference
      (bind _asgi_thesis (Utilities|Casting|CastToGI_Thesis (Game|GetGameInstance))
        (:then
          (Variables|Default|SetGameInstance _asgi_thesis))
        (:CastFailed
          (Development|PrintString "GI_Thesis cast failed!" true true "(R=0.651042,G=0.000000,B=0.000000,A=1.000000)" 5.0))))
    (:then_1
      (|LoadGameInstanceData))
    (:then_2
      ;[1 1 1] Set Temporary Point Pool as Current Point Pool
      (Variables|Temporary|SetTmpPointPool (Variables|Default|GetCurrentPointPool)))))

(event EventEndPlay
  (params (EndPlayReason :type EEndPlayReason%20Enum :default "Destroyed"))
  (if (Utilities|Enum|Equal(Enum) EndPlayReason "LevelTransition")
    (Utilities|FlowControl|Sequence
      (:then_0
        ;[1 1 1] Increase Level Counter
        (Math|Integer|IncrementInt (Variables|/Game/Blueprints/GI_Thesis.GI_Thesis_C|GetLevelCounter (Variables|Default|GetGameInstance))))
      (:then_1
        ;[1 1 1] Save CurrentPointPool
        (Variables|/Game/Blueprints/GI_Thesis.GI_Thesis_C|SetSavedPointPool (Variables|Default|GetGameInstance) (Variables|Default|GetCurrentPointPool)))
      (:then_2
        ;[1 1 1] Save CollectedCombatData
        (Variables|/Game/Blueprints/GI_Thesis.GI_Thesis_C|SetSavedCombatData (Variables|Default|GetGameInstance) (Variables|Default|GetCollectedCombatData))))))

(fn SaveCombatData
  (params (ActionCharacter :type BP%20Action%20Char%20Class%20Reference) (CombatData :type S%20Combat%20Data%20Structure))
  (bind (_array_element _array_index) (Utilities|Array|ForEachLoopwithBreak (Variables|Default|GetCollectedCombatData) :!label _label)
    (:LoopBody
      (if (== (.actioncharacter _array_element) ActionCharacter)
        (LocalVariables|SetEntryFound true)
        (Utilities|Array|Add (.combatdataarray (Utilities|Array|Get(acopy) (Variables|Default|GetCollectedCombatData) _array_index)) CombatData)
        (Development|PrintString "New CombatData entry added")
        (goto _label Break)))
    (:Completed
      (if (not (LocalVariables|GetEntryFound))
        (Utilities|Array|Add (Variables|Default|GetCollectedCombatData) (Utilities|Struct|MakeS_CollectedCombatData ActionCharacter (Utilities|Array|MakeArray CombatData)))
        (Development|PrintString "New CombatData Table added")))))

(fn DEBUGPrintCollectedCombatData
  (params (ActionCharacter :type BP%20Action%20Char%20Class%20Reference))
  (bind _array_element (Utilities|Array|ForEachLoopwithBreak (Variables|Default|GetCollectedCombatData) :!label _label)
    (:LoopBody
      (if (== (.actioncharacter _array_element) ActionCharacter)
        (for (_array_element_2 _array_index) (.combatdataarray _array_element)
          (Development|PrintText (Utilities|Text|FormatText "ActionCharacter = {acName} 
Record Nr. {index} 
Damage Received = {DR} 
Time To Kill = {TTK}" (Utilities|GetClassDisplayName ActionCharacter) _array_index (.damagereceived _array_element_2) (.timetokill _array_element_2))))
        (goto _label Break)))))