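; Game mode that populates Paper2D tile map levels with player, enemies and exit, and drives level progression.
; Construction caches tiles carrying user data; BeginPlay uses them as spawn markers.
; Enemy spawning spends ACScoringAgent's point pool on seeded random data-table picks, dropping unaffordable or too-cheap types and falling back to the priciest.
; AttemptLevelChange requires no remaining enemies (or a debug override), then increases the pool and opens the agent's next map.
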(event Custom|AttemptLevelChange
  (bind _ac_scoringagent (Variables|Default|GetAC_ScoringAgent))
  (bind _enemiesremaining (Variables|Default|GetEnemiesRemaining))
  (bind _returnvalue (Utilities|Set|Length _enemiesremaining))
  (if (or (<= _returnvalue 0) (Variables|Debug|GetDebugEndLevelActive))
    (Utilities|FlowControl|DoOnce false
      (:Completed
        (Default|IncreasePointPool _ac_scoringagent)
        (bind _world_asset (Default|FetchNextMap _ac_scoringagent))
        (Game|OpenLevel(byObjectReference) _world_asset)))
    (else
      (Development|PrintText (Utilities|Text|FormatText "Level not yet completed! 
Remaining Enemies - {length} 
" _returnvalue)))))

(event EventBeginPlay
  (Utilities|FlowControl|Sequence
    (:then_0
      (bind _asgi_thesis (Utilities|Casting|CastToGI_Thesis (Game|GetGameInstance)))
      (Variables|Default|SetGameInstance _asgi_thesis))
    (:then_1
      (Class|KismetMathLibrary|SeedRandomStream (Variables|Default|GetSeed)))
    (:then_2
      (CallFunction|SpawnPlayer (Variables|Default|GetMetadataTiles)))
    (:then_3
      (CallFunction|SpawnEnemies (Variables|Default|GetMetadataTiles)))
    (:then_4
      (CallFunction|SpawnLevelEnd (Variables|Default|GetMetadataTiles)))
    (:then_5
      ;[1 1 1] DEBUG
      (Development|PrintText (Utilities|Text|FormatText "Current Level Counter - {LC} 
" (Variables|/Game/Blueprints/GI_Thesis.GI_Thesis_C|GetLevelCounter (Variables|Default|GetGameInstance)))))))

(event Custom|FetchAllTilesInfo
  (bind _tilemapactor (Variables|Default|GetTileMapActor))
  (bind _rendercomponent (Variables|/Script/Paper2D.PaperTileMapActor|GetRenderComponent _tilemapactor))
  (bind (_mapwidth _mapheight) (Class|PaperTileMapComponent|GetMapSize _rendercomponent))
  (bind _index (Utilities|FlowControl|ForLoopwithBreak 0 (- _mapwidth 1))
    (:LoopBody
      (bind _index_2 (Utilities|FlowControl|ForLoopwithBreak 0 (- _mapheight 1))
        (:LoopBody
          (if (== (Class|TileMapBlueprintLibrary|GetTileUserData (Class|PaperTileMapComponent|GetTile _rendercomponent _index _index_2 2)) "PlayerStart")
            (Development|PrintText (Utilities|Text|FormatText "JACKPOT! 
 
Value Location X = {x} 
Value Location Y = {y} 
Value Location Z = {z}" (.x (Class|PaperTileMapComponent|GetTileCenterPosition _rendercomponent _index _index_2 2 true)) (.y (Class|PaperTileMapComponent|GetTileCenterPosition _rendercomponent _index _index_2 2 true)) (.z (Class|PaperTileMapComponent|GetTileCenterPosition _rendercomponent _index _index_2 2 true))))))))))

(fn ConstructionScript
  (Utilities|FlowControl|Sequence
    (:then_0
      (bind _returnvalue (Actor|GetActorOfClass "/Script/Paper2D.PaperTileMapActor"))
      (bind _output_get (Variables|Default|SetTileMapActor _returnvalue))
      (CallFunction|FetchMetadataTiles (Variables|/Script/Paper2D.PaperTileMapActor|GetRenderComponent _output_get)))))

(fn SpawnEnemies
  (params (MetadataTiles :type Array%20of%20S%20Tile%20Info%20Structures))
  (for _array_element MetadataTiles
    (if (== (Utilities|Struct|BreakS_TileInfo _array_element) "EnemySpawn")
      (Utilities|Array|AddUnique (LocalVariables|GetEnemyTiles) _array_element)))
  ;[1 0.8763 0.477] Spawn enemies according to rules
  (bind _outrownames (DataTable|GetDataTableRowNames (Variables|Default|GetEnemyValues)))
  (LocalVariables|SetEnemyRowNames _outrownames)
  (while (Math|Boolean|ANDBoolean (> (Utilities|GetCurrentPointPool) 0.0) (> (Utilities|Array|Length (LocalVariables|GetEnemyTiles)) 0) (> (Utilities|Array|Length (LocalVariables|GetEnemyRowNames)) 0))
    (LocalVariables|SetTmpRowName (.OutItem (Utilities|Array|RandomFromStream (LocalVariables|GetEnemyRowNames) (Variables|Default|GetSeed))))
    (bind _returnvalue (Utilities|GetDataTableRow (Variables|Default|GetEnemyValues) (LocalVariables|GetTmpRowName))
      (:then
        (LocalVariables|SetTmpRow _returnvalue)
        (if (>= (Utilities|GetCurrentPointPool) (.value (LocalVariables|GetTmpRow)))
          (|CompatibilityCheck
            (:then
              ;;[1 1 1] DEBUG
              (Development|PrintText (Utilities|Text|FormatText "Current Point Pool: {PointPool} 
Spawning {className} that costs {cost} points." (Utilities|GetCurrentPointPool) (Utilities|GetClassDisplayName (.actioncharacter (LocalVariables|GetTmpRow))) (.value (LocalVariables|GetTmpRow))))
              (Variables|/Game/PointSystem/AC_ScoringAgent.AC_ScoringAgent_C|SetTmpPointPool (Variables|Default|GetAC_ScoringAgent) (- (Utilities|GetCurrentPointPool) (.value (LocalVariables|GetTmpRow))))
              (bind _output_get (LocalVariables|SetTmpTile (.OutItem (Utilities|Array|RandomFromStream (LocalVariables|GetEnemyTiles) (Variables|Default|GetSeed)))))
              (bind _returnvalue_2 (Game|SpawnActorfromClass (.actioncharacter (LocalVariables|GetTmpRow)) (Math|Transform|MakeTransform (Math|Vector|MakeVector (.x (Class|PaperTileMapComponent|GetTileCenterPosition (.rendercomponent _output_get) (.x _output_get) (.y _output_get) (.layer _output_get) true)) 0.0 (.z (Class|PaperTileMapComponent|GetTileCenterPosition (.rendercomponent _output_get) (.x _output_get) (.y _output_get) (.layer _output_get) true))) (Transformation|GetWorldRotation (.rendercomponent _output_get)) "1.000000,1.000000,1.000000") "AlwaysSpawn" "MultiplyWithRoot" 0 0))
              (Utilities|Set|Add (Variables|Default|GetEnemiesRemaining) _returnvalue_2)
              (Utilities|Array|RemoveItem (LocalVariables|GetEnemyTiles) (LocalVariables|GetTmpTile))
              ;;[1 1 1] DEBUG
              (Development|PrintText (Utilities|Text|FormatText "Enemy Tiles left: {ET} 
Point Pool after spawn: {PP}" (Utilities|Array|Length (LocalVariables|GetEnemyTiles)) (Utilities|GetCurrentPointPool))))
            (:else
              (Utilities|Array|RemoveItem (LocalVariables|GetEnemyRowNames) (LocalVariables|GetTmpRowName) :!label _label)
              (Development|PrintText (Utilities|Text|FormatText "Not enough points for {RowName}. Removing from Enemy Row Names" (LocalVariables|GetTmpRowName)))))
          (else
            (goto _label))))
      (:RowNotFound
        (Development|PrintString "DT_EnemyValues Row Not Found!" true true "(R=1.000000,G=0.000000,B=0.012242,A=1.000000)" 5.0))))
  ;[1 0.1448 0.1846] Spawn highest cost enemies if possible enemy pool runs out
  (if (Math|Boolean|ANDBoolean (> (Utilities|GetCurrentPointPool) 0.0) (> (Utilities|Array|Length (LocalVariables|GetEnemyTiles)) 0) (<= (Utilities|Array|Length (LocalVariables|GetEnemyRowNames)) 0))
    (Utilities|FlowControl|Sequence
      (:then_0
        ;;[1 1 1] Find Enemies Highest Point Cost
        (for _array_element_2 (Default|GetEnemyValues (Variables|Default|GetAC_ScoringAgent))
          (if (> (.value _array_element_2) (LocalVariables|GetTmpHighestPoint))
            (LocalVariables|SetTmpHighestPoint (.value _array_element_2)))))
      (:then_1
        ;;[1 1 1] Find Enemies that have cost equal or higher to the found Highest Point Cost
        (bind _outrownames_2 (DataTable|GetDataTableRowNames (Variables|Default|GetEnemyValues)))
        (for _array_element_3 _outrownames_2
          (bind _returnvalue_3 (Utilities|GetDataTableRow (Variables|Default|GetEnemyValues) _array_element_3)
            (:then
              (if (>= (Utilities|Struct|BreakS_ActorValue _returnvalue_3) (LocalVariables|GetTmpHighestPoint))
                (Utilities|Array|AddUnique (LocalVariables|GetTmpRowArray) _returnvalue_3))))))
      (:then_2
        ;;[1 1 1] Spawn Enemies until spawn points runs out or Point Pool runs out
        (while (and (> (Utilities|GetCurrentPointPool) 0.0) (> (Utilities|Array|Length (LocalVariables|GetEnemyTiles)) 0))
          (LocalVariables|SetTmpRow (.OutItem (Utilities|Array|RandomFromStream (LocalVariables|GetTmpRowArray) (Variables|Default|GetSeed))))
          (Variables|/Game/PointSystem/AC_ScoringAgent.AC_ScoringAgent_C|SetTmpPointPool (Variables|Default|GetAC_ScoringAgent) (- (Utilities|GetCurrentPointPool) (.value (LocalVariables|GetTmpRow))))
          (bind _output_get_2 (LocalVariables|SetTmpTile (.OutItem (Utilities|Array|RandomFromStream (LocalVariables|GetEnemyTiles) (Variables|Default|GetSeed)))))
          (bind _returnvalue_4 (Game|SpawnActorfromClass (.actioncharacter (LocalVariables|GetTmpRow)) (Math|Transform|MakeTransform (Math|Vector|MakeVector (.x (Class|PaperTileMapComponent|GetTileCenterPosition (.rendercomponent _output_get_2) (.x _output_get_2) (.y _output_get_2) (.layer _output_get_2) true)) 0.0 (.z (Class|PaperTileMapComponent|GetTileCenterPosition (.rendercomponent _output_get_2) (.x _output_get_2) (.y _output_get_2) (.layer _output_get_2) true))) (Transformation|GetWorldRotation (.rendercomponent _output_get_2)) "1.000000,1.000000,1.000000") "AlwaysSpawn" "MultiplyWithRoot" 0 0))
          (Utilities|Set|Add (Variables|Default|GetEnemiesRemaining) _returnvalue_4)
          (Utilities|Array|RemoveItem (LocalVariables|GetEnemyTiles) (LocalVariables|GetTmpTile))
          (Development|PrintText (Utilities|Text|FormatText "Enemy Tiles left: {ET} 
Point Pool after spawn: {PP}" (Utilities|Array|Length (LocalVariables|GetEnemyTiles)) (Utilities|GetCurrentPointPool))))
        (if (> (Utilities|GetCurrentPointPool) 0.0)
          (Development|PrintString "[WARNING] Maximum difficulty level reached! This prototype lacks implementation for excess Points and excess Points are ignored." true true "(R=1.000000,G=0.930875,B=0.000000,A=1.000000)"))))))

(fn FetchMetadataTiles
  (params (RenderComponent :type Paper%20Tile%20Map%20Component%20Object%20Reference))
  (bind (_mapwidth _mapheight _numlayers) (Class|PaperTileMapComponent|GetMapSize RenderComponent))
  (for _index (range 0 (- _mapwidth 1))
    (for _index_2 (range 0 (- _mapheight 1))
      (for _index_3 (range 0 (- _numlayers 1))
        (if (!= (Class|TileMapBlueprintLibrary|GetTileUserData (Class|PaperTileMapComponent|GetTile RenderComponent _index _index_2 _index_3)) "")
          (Utilities|Array|AddUnique (Variables|Default|GetMetadataTiles) (Utilities|Struct|MakeS_TileInfo RenderComponent _index _index_2 _index_3 (Class|TileMapBlueprintLibrary|GetTileUserData (Class|PaperTileMapComponent|GetTile RenderComponent _index _index_2 _index_3)))))))))

(fn SpawnPlayer
  (params (MetadataTiles :type Array%20of%20S%20Tile%20Info%20Structures))
  (bind _array_element (Utilities|Array|ForEachLoopwithBreak MetadataTiles :!label _label)
    (:LoopBody
      (if (== (.userdata _array_element) "PlayerStart")
        (Transformation|Teleport (Game|GetPlayerCharacter 0) (Math|Vector|MakeVector (.x (Class|PaperTileMapComponent|GetTileCenterPosition (.rendercomponent _array_element) (.x _array_element) (.y _array_element) (.layer _array_element) true)) 0.0 (.z (Class|PaperTileMapComponent|GetTileCenterPosition (.rendercomponent _array_element) (.x _array_element) (.y _array_element) (.layer _array_element) true))) (Transformation|GetWorldRotation (.rendercomponent _array_element)))
        (goto _label Break)))))

(fn SpawnLevelEnd
  (params (MetadataTiles :type Array%20of%20S%20Tile%20Info%20Structures))
  (for _array_element MetadataTiles
    (if (== (.userdata _array_element) "LevelEnd")
      (Game|SpawnActorfromClass "/Game/Blueprints/BP_LevelEnd.BP_LevelEnd_C" (Math|Transform|MakeTransform (Math|Vector|MakeVector (.x (Class|PaperTileMapComponent|GetTileCenterPosition (.rendercomponent _array_element) (.x _array_element) (.y _array_element) (.layer _array_element) true)) 0.0 (.z (Class|PaperTileMapComponent|GetTileCenterPosition (.rendercomponent _array_element) (.x _array_element) (.y _array_element) (.layer _array_element) true))) (Transformation|GetWorldRotation (.rendercomponent _array_element)) "1.000000,1.000000,1.000000") "AlwaysSpawn" "MultiplyWithRoot" 0 0))))