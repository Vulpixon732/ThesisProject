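; BP_Shark is a shark enemy that targets the Captain on entering its aggro range, via its AI controller.
; It extends parent damage and attack logic, reporting combat start and damage dealt to an enemy-watcher component for a scoring agent.
; On defeat it moves its sprite to a defeated position, ends and sends combat data, and removes itself from the game mode's remaining enemies.
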(event OnComponentBeginOverlap(AggroRange)
  (params (OverlappedComponent :type Primitive%20Component%20Object%20Reference) (OtherActor :type Actor%20Object%20Reference) (OtherComp :type Primitive%20Component%20Object%20Reference) (OtherBodyIndex :type Integer) (bFromSweep :type Boolean) (SweepResult :type Hit%20Result%20Structure%20%28by%20ref%29))
  (bind _asbp_captain (Utilities|Casting|CastToBP_Captain OtherActor))
  (bind _asaic_enemy (Utilities|Casting|CastToAIC_Enemy (AI|GetAIController self)))
  (Default|SetAttackTarget _asaic_enemy _asbp_captain)
  ;[1 1 1] ScoringAgent - Measure time once Aggro is locked
  (if (not (Variables|Default|GetIsDefeated))
    (Default|BeginCombat (Variables|Default|GetAC_EnemyWatcher))))

(event Custom|OnDefeated
  (Transformation|SetRelativeLocation (Variables|Default|GetSprite) (Variables|/Script/Engine.SceneComponent|GetRelativeLocation (Variables|Default|GetDefeatedPos)) false false)
  ;[1 1 1] ScoringAgent - End Combat and send Combat Data after death
  (Default|EndCombat (Variables|Default|GetAC_EnemyWatcher))
  (Default|SendData (Variables|Default|GetAC_EnemyWatcher))
  ;[1 0.1132 0] Remove Self from Remaining Enemies list in Game Mode
  (bind _asgm_thesis (Utilities|Casting|CastToGM_Thesis (Game|GetGameMode)))
  (Utilities|Set|Remove (Variables|/Game/Blueprints/GM_Thesis.GM_Thesis_C|GetEnemiesRemaining _asgm_thesis) self))

(event EventBeginPlay
  (|CallParentFunction)
  (EventDispatchers|BindEventtoDefeated (delegate Custom|OnDefeated)))

(event Collision|EventActorBeginOverlap
  (params (OtherActor :type Actor%20Object%20Reference)))

(event EventTick
  (params (DeltaSeconds :type Float%20%28single-precision%29)))

(fn ConstructionScript
  (|CallParentFunction))

(fn DamageCharacter
  (params (Object :type Object%20Object%20Reference))
  (bind _succesful (|CallParentFunction Object))
  ;[1 1 1] ScoringAgent - Note down damage dealt to Player
  (if _succesful
    (Default|DealtDamagetoPlayer (Variables|Default|GetAC_EnemyWatcher) (Variables|Default|GetDamage)))
  (return _succesful))

(fn ReceiveAttack
  (params (Damage :type Float%20%28double-precision%29))
  (|CallParentFunction Damage)
  ;[1 1 1] ScoringAgent - Begin TimeToKill timer after receiving damage
  (if (not (Variables|Default|GetIsDefeated))
    (Default|BeginCombat (Variables|Default|GetAC_EnemyWatcher))))